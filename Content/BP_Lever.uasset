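; BP_Lever is an interactable lever that works as an on/off switch.
; On Interact it prints a debug message, flips its IsOn state and passes the new value to SendSignal.
; BeginPlay, overlap and Tick are unused stubs, and the construction script only calls its parent.
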(event EventBeginPlay
  (|CallParentFunction) ; This node is disabled and will not be called.\nDrag off pins to build functionality.
)

(event Collision|EventActorBeginOverlap
  (params (OtherActor :type Actor%20Object%20Reference))
  (|CallParentFunction OtherActor) ; This node is disabled and will not be called.\nDrag off pins to build functionality.
)

(event EventTick
  (params (DeltaSeconds :type Float%20%28single-precision%29))
  (|CallParentFunction DeltaSeconds) ; This node is disabled and will not be called.\nDrag off pins to build functionality.
)

(event EventInteract
  (Development|PrintString "Lever Hit" true true "(R=1.000000,G=0.081140,B=0.000000,A=1.000000)")
  (bind _output_get (Variables|Default|SetIsOn (not (Variables|Default|GetIsOn))))
  (CallFunction|SendSignal _output_get))

(fn ConstructionScript
  (|CallParentFunction))