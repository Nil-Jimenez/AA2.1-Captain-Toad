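; Switchable elevator platform that raises its Elevator component by RiseHeight and lowers it back.
; BeginPlay caches the component's starting relative location.
; SwitchON plays ElevatorTimeline and SwitchOFF reverses it, with the timeline's Alpha scaling a vertical offset from that start, without sweep.
; The OnSwitchedOn and OnSwitchedOff functions only call their parent versions.
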(event EventBeginPlay
  (Variables|Default|SetStartLocation (Variables|/Script/Engine.SceneComponent|GetRelativeLocation (Variables|Default|Getelevator))))

(event Collision|EventActorBeginOverlap
  (params (OtherActor :type Actor%20Object%20Reference))
  (|CallParentFunction OtherActor) ; This node is disabled and will not be called.\nDrag off pins to build functionality.
)

(event EventTick
  (params (DeltaSeconds :type Float%20%28single-precision%29))
  (|CallParentFunction DeltaSeconds) ; This node is disabled and will not be called.\nDrag off pins to build functionality.
)

(event EventSwitchOFF
  (bind _startlocation (Variables|Default|GetStartLocation))
  (bind (_x _y _z) (Math|Vector|BreakVector _startlocation))
  (bind _alpha (Timeline|ElevatorTimeline Reverse)
    (:Update
      (Transformation|SetRelativeLocation (Variables|Default|Getelevator) (Math|Vector|MakeVector _x _y (+ (* (Variables|Default|GetRiseHeight) _alpha) _z)) false false))))

(event EventSwitchON
  (bind _startlocation (Variables|Default|GetStartLocation))
  (bind (_x _y _z) (Math|Vector|BreakVector _startlocation))
  (bind _alpha (Timeline|ElevatorTimeline Play)
    (:Update
      (Transformation|SetRelativeLocation (Variables|Default|Getelevator) (Math|Vector|MakeVector _x _y (+ (* (Variables|Default|GetRiseHeight) _alpha) _z)) false false))))

(fn ConstructionScript
  (|CallParentFunction))

(fn OnSwitchedon
  (|CallParentFunction))

(fn OnSwitchedOff
  (|CallParentFunction))