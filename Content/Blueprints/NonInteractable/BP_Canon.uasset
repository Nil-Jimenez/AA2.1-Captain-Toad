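; BP_Canon is a switchable cannon that repeatedly fires BP_Bullet actors while switched on.
; Switching on fires immediately and starts a looping timer that calls Fire every FireInterval; switching off clears that timer.
; Fire spawns each bullet at the Muzzle transform with the cannon as owner, regardless of collisions.
; Both switch handlers pass through to the parent class, and no Tick logic is used.
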(event EventBeginPlay
  (|CallParentFunction) ; This node is disabled and will not be called.\nDrag off pins to build functionality.
)

(event Collision|EventActorBeginOverlap
  (params (OtherActor :type Actor%20Object%20Reference))
  (|CallParentFunction OtherActor) ; This node is disabled and will not be called.\nDrag off pins to build functionality.
)

(event EventTick
  (params (DeltaSeconds :type Float%20%28single-precision%29))
  (|CallParentFunction DeltaSeconds) ; This node is disabled and will not be called.\nDrag off pins to build functionality.
)

(fn ConstructionScript
  (|CallParentFunction))

(fn Fire
  (Game|SpawnActorfromClass "/Game/Blueprints/BP_Bullet.BP_Bullet_C" (Transformation|GetWorldTransform (Variables|Default|GetMuzzle)) "AlwaysSpawn" "MultiplyWithRoot" self 0))

(fn OnSwitchedon
  (CallFunction|Fire)
  (bind _returnvalue (Utilities|Time|SetTimerbyFunctionName 0 "Fire" (Variables|Default|GetFireInterval) true))
  (Variables|Default|SetFireTimer _returnvalue)
  (|CallParentFunction))

(fn OnSwitchedOff
  (Utilities|Time|ClearandInvalidateTimerbyHandle (Variables|Default|GetFireTimer))
  (|CallParentFunction))