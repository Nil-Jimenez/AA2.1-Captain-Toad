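; BP_ElevatorWithLever is an elevator actor paired with a lever embedded as a child actor.
; On BeginPlay it casts the LeverChild actor to BP_Lever and adds itself to that lever's EnabledActors, so the link is made at runtime.
; The construction script only calls the parent, and no movement logic appears in these graphs.
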(event EventBeginPlay
  (bind _asbp_lever (Utilities|Casting|CastToBP_Lever (Variables|/Script/Engine.ChildActorComponent|GetChildActor (Variables|Default|GetLeverChild))))
  (Utilities|Array|Add (Variables|/Game/Blueprints/Interactable/BP_InteractableObject.BP_InteractableObject_C|GetEnabled%20Actors _asbp_lever) self))

(event Collision|EventActorBeginOverlap
  (params (OtherActor :type Actor%20Object%20Reference))
  (|CallParentFunction OtherActor) ; This node is disabled and will not be called.\nDrag off pins to build functionality.
)

(event EventTick
  (params (DeltaSeconds :type Float%20%28single-precision%29))
  (|CallParentFunction DeltaSeconds) ; This node is disabled and will not be called.\nDrag off pins to build functionality.
)

(fn ConstructionScript
  (|CallParentFunction))