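; BP_Padlock is an interactable lock that a BP_Key actor opens by touching its KeyZone.
; On a key overlap while still closed, it destroys the key, marks itself opened and on, hides itself and disables collision on both KeyZone and Lock.
; It then calls SendSignal with the on state, and the Opened flag keeps this from repeating.
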(event OnComponentBeginOverlap(KeyZone)
  (params (OverlappedComponent :type Primitive%20Component%20Object%20Reference) (OtherActor :type Actor%20Object%20Reference) (OtherComp :type Primitive%20Component%20Object%20Reference) (OtherBodyIndex :type Integer) (bFromSweep :type Boolean) (SweepResult :type Hit%20Result%20Structure%20%28by%20ref%29))
  (if (not (Variables|Default|GetbOpened))
    (bind _asbp_key (Utilities|Casting|CastToBP_Key OtherActor))
    (Actor|DestroyActor _asbp_key)
    (Variables|Default|SetbOpened true)
    (bind _output_get (Variables|Default|SetIsOn true))
    (Rendering|SetActorHiddenInGame _output_get)
    (Collision|SetCollisionEnabled (Variables|Default|GetKeyZone) "NoCollision")
    (Collision|SetCollisionEnabled (Variables|Default|Getlock) "NoCollision")
    (CallFunction|SendSignal _output_get)))

(event EventBeginPlay
  (|CallParentFunction) ; This node is disabled and will not be called.\nDrag off pins to build functionality.
)

(event Collision|EventActorBeginOverlap
  (params (OtherActor :type Actor%20Object%20Reference))
  (|CallParentFunction OtherActor) ; This node is disabled and will not be called.\nDrag off pins to build functionality.
)

(event EventTick
  (params (DeltaSeconds :type Float%20%28single-precision%29))
  (|CallParentFunction DeltaSeconds) ; This node is disabled and will not be called.\nDrag off pins to build functionality.
)

(fn ConstructionScript
  (|CallParentFunction))