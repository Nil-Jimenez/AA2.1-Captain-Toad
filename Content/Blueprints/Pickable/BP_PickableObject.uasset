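; BP_PickableObject is a physics object that can be picked up, carried and dropped.
; PickUp flags it as held, stops physics simulation, sets the mesh to query-only collision and snaps it onto the supplied Carrier component.
; Drop detaches it in world space, nudges it along its own forward vector without a sweep, then restores collision and physics and clears the held flag.
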(event EventBeginPlay)

(event Collision|EventActorBeginOverlap
  (params (OtherActor :type Actor%20Object%20Reference)))

(event EventTick
  (params (DeltaSeconds :type Float%20%28single-precision%29)))

(fn ConstructionScript)

(fn PickUp
  (params (Carrier :type Scene%20Component%20Object%20Reference))
  (Variables|Default|SetbIsHeld true)
  (Physics|SetSimulatePhysics (Variables|Default|GetMesh) false)
  (Collision|SetCollisionEnabled (Variables|Default|GetMesh) "QueryOnly")
  (Transformation|AttachComponentToComponent Carrier "None" "SnapToTarget" "SnapToTarget" "SnapToTarget" true))

(fn Drop
  (Transformation|DetachFromActor "KeepWorld" "KeepWorld" "KeepWorld")
  (Transformation|SetActorLocation (+ (Transformation|GetActorLocation) (* (Transformation|GetActorForwardVector) 100)) false false)
  (Collision|SetCollisionEnabled (Variables|Default|GetMesh) "QueryAndPhysics")
  (Physics|SetSimulatePhysics (Variables|Default|GetMesh) true)
  (Variables|Default|SetbIsHeld false))