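; BP_CounterComponent is a counter component that restarts the current level once its count reaches a fixed threshold of five.
; AddAmount adds the given amount to Count and, at or above the threshold, reopens the current level by name.
; Below the threshold, it broadcasts the new value through the OnCountChanged dispatcher.
; BeginPlay and Tick are unused, so all logic runs only when AddAmount is called.
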(event EventBeginPlay)

(event EventTick
  (params (DeltaSeconds :type Float%20%28single-precision%29)))

(fn AddAmount
  (params (Amount :type Integer))
  (Variables|Default|SetCount (+ Amount (Variables|Default|GetCount)))
  (if (>= (Variables|Default|GetCount) 5)
    (bind _returnvalue (Game|GetCurrentLevelName true))
    (Game|OpenLevel(byName) (Utilities|String|StringToName _returnvalue))
    (else
      (Default|CallOnCountChanged (Variables|Default|GetCount)))))