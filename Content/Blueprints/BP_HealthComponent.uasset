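; BP_HealthComponent is an actor component that tracks an integer health value for its owner.
; It starts at MaxHealth and binds to the owner's TakeAnyDamage, truncating damage into RemoveHealth.
; AddHealth and RemoveHealth clamp the value between zero and max and broadcast OnHealthChanged.
; RemoveHealth ignores hits once health is zero and fires OnDeath when it reaches zero.
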(event Custom|OnTakeAnyDamage_Event
  (params (DamagedActor :type Actor%20Object%20Reference) (Damage :type Float%20%28single-precision%29) (DamageType :type Damage%20Type%20Object%20Reference) (InstigatedBy :type Controller%20Object%20Reference) (DamageCauser :type Actor%20Object%20Reference))
  (CallFunction|RemoveHealth (Math|Float|Truncate Damage)))

(event EventBeginPlay
  (Variables|Default|SetCurrentHealth (Variables|Default|GetMaxHealth))
  (EventDispatchers|AssignOnTakeAnyDamage (Components|GetOwner) (delegate Custom|OnTakeAnyDamage_Event)))

(event EventTick
  (params (DeltaSeconds :type Float%20%28single-precision%29)))

(fn AddHealth
  (params (Amount :type Integer))
  (Variables|Default|SetCurrentHealth (Math|Integer|Clamp(Integer) (+ (Variables|Default|GetCurrentHealth) Amount) 0 (Variables|Default|GetMaxHealth)))
  (Default|CallOnHealthChanged (Variables|Default|GetCurrentHealth) (Variables|Default|GetMaxHealth)))

(fn RemoveHealth
  (params (Amount :type Integer))
  (if (> (Variables|Default|GetCurrentHealth) 0)
    (Variables|Default|SetCurrentHealth (Math|Integer|Clamp(Integer) (- (Variables|Default|GetCurrentHealth) Amount) 0 (Variables|Default|GetMaxHealth)))
    (Default|CallOnHealthChanged (Variables|Default|GetCurrentHealth) (Variables|Default|GetMaxHealth))
    (if (<= (Variables|Default|GetCurrentHealth) 0)
      (Default|CallOnDeath))))