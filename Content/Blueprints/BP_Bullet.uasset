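; BP_Bullet is a projectile actor that damages what it hits or sets off a physics impulse.
; On BeginPlay its collision component ignores the owning actor while moving.
; On hit, it applies damage to actors that have a BP_HealthComponent, and otherwise fires the Explosion component's impulse.
; The bullet destroys itself in both cases.
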(event OnComponentHit(Collision)
  (params (HitComponent :type Primitive%20Component%20Object%20Reference) (OtherActor :type Actor%20Object%20Reference) (OtherComp :type Primitive%20Component%20Object%20Reference) (NormalImpulse :type Vector :default "0, 0, 0") (Hit :type Hit%20Result%20Structure%20%28by%20ref%29))
  (Utilities|IsValid (Actor|GetComponentbyClass OtherActor "/Game/Blueprints/BP_HealthComponent.BP_HealthComponent_C")
    (:Is%20Valid
      (Game|Damage|ApplyDamage OtherActor 1.0 0 self)
      (Actor|DestroyActor))
    (:Is%20Not%20Valid
      (Class|RadialForceComponent|FireImpulse (Variables|Default|GetExplosion))
      (Actor|DestroyActor))))

(event EventBeginPlay
  (Collision|IgnoreActorwhenMoving (Variables|Default|GetCollision) (Components|GetOwner) true))

(event Collision|EventActorBeginOverlap
  (params (OtherActor :type Actor%20Object%20Reference)))

(event EventTick
  (params (DeltaSeconds :type Float%20%28single-precision%29)))

(fn ConstructionScript)