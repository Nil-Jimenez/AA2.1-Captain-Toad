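; Switchable platform that rotates around its yaw axis when turned on or off.
; Switch-on targets RotationAngle from the start yaw if UndoOnOff is set, otherwise from the last target; switch-off always returns to the start yaw.
; RotateTo captures the current yaw and plays a timeline whose alpha blends toward the target, so a new call continues from wherever the platform is.
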(event Custom|RotateTo
  (params (NewTargetYaw :type Float%20%28double-precision%29))
  (Variables|Default|SetTargetYaw NewTargetYaw)
  (Variables|Default|SetBaseYaw (Variables|Default|GetCurrentYaw))
  (Variables|Default|SetYawDelta (- NewTargetYaw (Variables|Default|GetBaseYaw)))
  (bind _alpha (Timeline|RotTimeline PlayFromStart)
    (:Update
      (bind _output_get (Variables|Default|SetCurrentYaw (+ (* (Variables|Default|GetYawDelta) _alpha) (Variables|Default|GetBaseYaw))))
      (Transformation|SetRelativeRotation (Variables|Default|Getplatform) (Math|Rotator|MakeRotator 0.0 0.0 _output_get) false false))))

(event EventBeginPlay
  (Variables|Default|SetStartYaw (.Yaw (Math|Rotator|BreakRotator (Variables|/Script/Engine.SceneComponent|GetRelativeRotation (Variables|Default|Getplatform)))))
  (Variables|Default|SetTargetYaw (Variables|Default|GetStartYaw))
  (Variables|Default|SetCurrentYaw (Variables|Default|GetStartYaw)))

(event Collision|EventActorBeginOverlap
  (params (OtherActor :type Actor%20Object%20Reference))
  (|CallParentFunction OtherActor) ; This node is disabled and will not be called.\nDrag off pins to build functionality.
)

(event EventTick
  (params (DeltaSeconds :type Float%20%28single-precision%29))
  (|CallParentFunction DeltaSeconds) ; This node is disabled and will not be called.\nDrag off pins to build functionality.
)

(event EventSwitchON
  (CallFunction|OnSwitchedon))

(event EventSwitchOFF
  (CallFunction|OnSwitchedOff))

(fn ConstructionScript
  (|CallParentFunction))

(fn OnSwitchedOff
  (if true
    (CallFunction|Rotateto (Variables|Default|GetStartYaw))
    (|CallParentFunction)))

(fn OnSwitchedon
  (if (Variables|Default|GetbUndoOnOff)
    (CallFunction|Rotateto (+ (Variables|Default|GetStartYaw) (Variables|Default|GetRotationAngle)))
    (else
      (CallFunction|Rotateto (+ (Variables|Default|GetTargetYaw) (Variables|Default|GetRotationAngle)))))
  (|CallParentFunction))