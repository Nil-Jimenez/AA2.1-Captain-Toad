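; Switchable door actor that shows an open or closed state by swapping the static mesh on its door mesh component.
; It starts with the closed mesh on BeginPlay.
; SwitchON and SwitchOFF events call OnSwitchedOn and OnSwitchedOff, which set the open or closed mesh and then call their parent implementations.
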(event EventBeginPlay
  (Components|StaticMesh|SetStaticMesh (Variables|Default|GetDoorMesh) (Variables|Default|GetClosedMesh)))

(event Collision|EventActorBeginOverlap
  (params (OtherActor :type Actor%20Object%20Reference))
  (|CallParentFunction OtherActor) ; This node is disabled and will not be called.\nDrag off pins to build functionality.
)

(event EventTick
  (params (DeltaSeconds :type Float%20%28single-precision%29))
  (|CallParentFunction DeltaSeconds) ; This node is disabled and will not be called.\nDrag off pins to build functionality.
)

(event EventSwitchON
  (CallFunction|OnSwitchedon))

(event EventSwitchOFF
  (CallFunction|OnSwitchedOff))

(fn ConstructionScript
  (|CallParentFunction))

(fn OnSwitchedOff
  (Components|StaticMesh|SetStaticMesh (Variables|Default|GetDoorMesh) (Variables|Default|GetClosedMesh))
  (|CallParentFunction))

(fn OnSwitchedon
  (Components|StaticMesh|SetStaticMesh (Variables|Default|GetDoorMesh) (Variables|Default|GetOpenMesh))
  (|CallParentFunction))