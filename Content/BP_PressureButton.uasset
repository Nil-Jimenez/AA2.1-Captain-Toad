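; Pressure button that toggles on or off based on the mass of physics objects in its trigger zone and sends that state as a signal.
; Each overlap begin or end sums the mass of simulating components and flips IsOn whenever it meets MassThreshold.
; A timeline then plays or reverses with IsOn, lerping the button mesh's Z scale to show it pressed.
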(event OnComponentBeginOverlap(TriggerZone)
  (params (OverlappedComponent :type Primitive%20Component%20Object%20Reference) (OtherActor :type Actor%20Object%20Reference) (OtherComp :type Primitive%20Component%20Object%20Reference) (OtherBodyIndex :type Integer) (bFromSweep :type Boolean) (SweepResult :type Hit%20Result%20Structure%20%28by%20ref%29))
  (bind _startscale (Variables|Default|GetStartScale))
  (bind (_x _y _z) (Math|Vector|BreakVector _startscale))
  (Development|PrintString "Presionado")
  (CallFunction|UpdatePressure)
  (if (Variables|Default|GetIsOn)
    (bind _alpha (Timeline|PressTimeLine Play)
      (:Update
        (Transformation|SetRelativeScale3D (Variables|Default|Getbutton-square) (Math|Vector|MakeVector _x _y (+ _z (Math|Float|Lerp 0.0 (* (Variables|Default|GetPressDepth) -0.3) _alpha))))))
    (else
      (Timeline|PressTimeLine Reverse))))

(event OnComponentEndOverlap(TriggerZone)
  (params (OverlappedComponent :type Primitive%20Component%20Object%20Reference) (OtherActor :type Actor%20Object%20Reference) (OtherComp :type Primitive%20Component%20Object%20Reference) (OtherBodyIndex :type Integer))
  (bind _startscale (Variables|Default|GetStartScale))
  (bind (_x _y _z) (Math|Vector|BreakVector _startscale))
  (Development|PrintString "No Presionado")
  (CallFunction|UpdatePressure)
  (if (Variables|Default|GetIsOn)
    (bind _alpha (Timeline|PressTimeLine Play)
      (:Update
        (Transformation|SetRelativeScale3D (Variables|Default|Getbutton-square) (Math|Vector|MakeVector _x _y (+ _z (Math|Float|Lerp 0.0 (* (Variables|Default|GetPressDepth) -0.3) _alpha))))))
    (else
      (Timeline|PressTimeLine Reverse))))

(event EventBeginPlay
  (Transformation|SetRelativeScale3D (Variables|Default|Getbutton-square) "1.000000,1.000000,1.700000")
  (Variables|Default|SetStartScale "1.000000,1.000000,1.700000"))

(event Collision|EventActorBeginOverlap
  (params (OtherActor :type Actor%20Object%20Reference))
  (|CallParentFunction OtherActor) ; This node is disabled and will not be called.\nDrag off pins to build functionality.
)

(event EventTick
  (params (DeltaSeconds :type Float%20%28single-precision%29))
  (|CallParentFunction DeltaSeconds) ; This node is disabled and will not be called.\nDrag off pins to build functionality.
)

(fn ConstructionScript
  (|CallParentFunction))

(fn UpdatePressure
  (for _array_element (Class|PrimitiveComponent|GetOverlappingComponents (Variables|Default|GetTriggerZone))
    (if (Physics|IsSimulatingPhysics _array_element "None")
      (LocalVariables|SetTotalMass (+ (Physics|GetMass _array_element) (LocalVariables|GetTotalMass)))))
  (if (>= (LocalVariables|GetTotalMass) (Variables|Default|GetMassThreshold))
    (bind _output_get (Variables|Default|SetIsOn (!= (>= (LocalVariables|GetTotalMass) (Variables|Default|GetMassThreshold)) (Variables|Default|GetIsOn))))
    (CallFunction|SendSignal _output_get)))